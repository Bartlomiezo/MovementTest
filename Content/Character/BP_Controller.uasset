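; Player controller that sets up Enhanced Input, moves the controlled pawn and handles pausing.
; BeginPlay adds the character and uneditable mapping contexts, registering the character one with user settings.
; Movement input maps to diagonal world axes, independent of camera rotation.
; Two IA_Pause handlers act separately: one lazily creates and toggles WB_Pause with the input mode, the other flip-flops game pause without checking menu visibility.
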(event Input|EnhancedActionEvents|EnhancedInputActionIA_Pause
  (params (ActionValue :type Boolean) (ElapsedSeconds :type Float%20%28double-precision%29) (TriggeredSeconds :type Float%20%28double-precision%29) (InputAction :type Input%20Action%20Object%20Reference :default "/Game/Character/IA_Pause.IA_Pause"))
  (:Completed
    (Utilities|FlowControl|FlipFlop
      (:A
        (Game|SetGamePaused (Variables|Default|GetPaused)))
      (:B
        (Game|SetGamePaused (Variables|Default|GetUnPaused))))))

(event Input|EnhancedActionEvents|EnhancedInputActionIA_Pause
  (params (ActionValue :type Boolean) (ElapsedSeconds :type Float%20%28double-precision%29) (TriggeredSeconds :type Float%20%28double-precision%29) (InputAction :type Input%20Action%20Object%20Reference :default "/Game/Character/IA_Pause.IA_Pause"))
  (bind _returnvalue (Game|GetPlayerController 0))
  (:Completed
    (Utilities|IsValid (Variables|Default|GetWB_PauseRef)
      (:Is%20Valid
        (if (Widget|IsVisible (Variables|Default|GetWB_PauseRef))
          (Widget|RemovefromParent (Variables|Default|GetWB_PauseRef))
          (Input|SetInputModeGameOnly _returnvalue false)
          (Variables|/Script/Engine.PlayerController|SetbShowMouseCursor _returnvalue true)
          (else
            (UserInterface|Viewport|AddtoViewport (stale _output_get) 0 :!label _label)
            (Input|SetInputModeGameandUI (Game|GetPlayerController 0) (stale _output_get) "DoNotLock" false false))))
      (:Is%20Not%20Valid
        (bind _returnvalue_2 (UserInterface|CreateWidget "/Game/Widgets/WB_Pause.WB_Pause_C" 0 0))
        (bind _output_get (Variables|Default|SetWB_PauseRef _returnvalue_2))
        (goto _label)))))

(event Input|EnhancedActionEvents|EnhancedInputActionIA_Movement
  (params (ActionValue :type Vector%202D%20Structure) (ElapsedSeconds :type Float%20%28double-precision%29) (TriggeredSeconds :type Float%20%28double-precision%29) (InputAction :type Input%20Action%20Object%20Reference :default "/Game/Character/IA_Movement.IA_Movement"))
  (bind _returnvalue (Pawn|GetControlledPawn))
  (Pawn|Input|AddMovementInput _returnvalue "1.000000,1.000000,0.000000" (.x ActionValue) false)
  (Pawn|Input|AddMovementInput _returnvalue "1.000000,-1.000000,0.000000" (.y ActionValue) false))

(event EventBeginPlay
  (bind _returnvalue (PlayerController|LocalPlayerSubsystems|GetEnhancedInputLocalPlayerSubsystem))
  (bind _returnvalue_2 (Class|EnhancedInputSubsystemInterface|GetUserSettings _returnvalue))
  (Utilities|IsValid _returnvalue
    (:Is%20Valid
      (Input|AddMappingContext _returnvalue "/Game/Character/IM_Character.IM_Character" 0 "(bIgnoreAllPressedKeysUntilRelease=True,bForceImmediately=False,bNotifyUserSettings=False)")
      (Input|AddMappingContext _returnvalue "/Game/Character/IM_Uneditable.IM_Uneditable" 0 "(bIgnoreAllPressedKeysUntilRelease=True,bForceImmediately=False,bNotifyUserSettings=False)")
      (if (not (Class|EnhancedInputUserSettings|IsMappingContextRegistered _returnvalue_2 "/Game/Character/IM_Character.IM_Character"))
        (Class|EnhancedInputUserSettings|RegisterInputMappingContext _returnvalue_2 "/Game/Character/IM_Character.IM_Character")))))

(event EventTick
  (params (DeltaSeconds :type Float%20%28single-precision%29)))

(fn ConstructionScript)